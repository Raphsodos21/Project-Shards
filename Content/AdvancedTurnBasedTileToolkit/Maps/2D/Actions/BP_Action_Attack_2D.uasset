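; 2D attack action for the turn-based tile toolkit that plays a unit's attack on a target visually and audibly.
; On BeginPlay it takes sounds and puppets from the units, plus a projectile sprite if the attacker's range exceeds one.
; With a projectile it spawns BP_Projectile and binds its hit event; otherwise a timeline lerps the attacker toward the target in XY.
; Either path calls AttackHit, which plays the hit sound and ends the action.
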(event Custom|AttackHit
  (Audio|PlaySound2D (Variables|Default|GetHitSound) 1.0 1.0 0.0 0 0)
  (CallFunction|EndAction true))

(event Custom|MeleeStrike
  (bind ___ (Utilities|MakeLocalVariable (Transformation|GetActorLocation (Variables|Default|GetSourcePuppet))))
  (bind _movetrack (Timeline|TL_Strike PlayFromStart)
    (:Update
      (Transformation|SetActorLocation (Variables|Default|GetSourcePuppet) (Math|Vector|MakeVector (.x (Math|Vector|Lerp(Vector) ___ (Transformation|GetActorLocation (Variables|Default|GetTargetPuppet)) _movetrack)) (.y (Math|Vector|Lerp(Vector) ___ (Transformation|GetActorLocation (Variables|Default|GetTargetPuppet)) _movetrack)) (.Z (Math|Vector|BreakVector ___))) false false))
    (:Strike
      (CallFunction|AttackHit))))

(event EventBeginPlay
  (bind _sourceunit2d (Variables|Default|GetSourceUnit2D))
  (bind _sourceunit2d_2 (Variables|Default|GetSourceUnit2D))
  (Variables|Default|SetAttackSound (Variables|/Game/AdvancedTurnBasedTileToolkit/Maps/2D/Units/BP_Unit_2D.BP_Unit_2D_C|GetAttackSound _sourceunit2d_2))
  (Variables|Default|SetProjectile (select (> (Variables|/Game/AdvancedTurnBasedTileToolkit/Core/Units/BP_Unit.BP_Unit_C|GetRange _sourceunit2d_2) 1) (Variables|/Game/AdvancedTurnBasedTileToolkit/Maps/2D/Units/BP_Unit_2D.BP_Unit_2D_C|GetProjectile _sourceunit2d_2) 0))
  (Variables|Default|SetHitSound (Variables|/Game/AdvancedTurnBasedTileToolkit/Maps/2D/Units/BP_Unit_2D.BP_Unit_2D_C|GetHitSound _sourceunit2d))
  (Variables|Default|SetSourcePuppet (Variables|/Game/AdvancedTurnBasedTileToolkit/Core/Units/BP_Unit.BP_Unit_C|GetPuppet _sourceunit2d))
  (Variables|Default|SetTargetPuppet (Variables|/Game/AdvancedTurnBasedTileToolkit/Core/Units/BP_Unit.BP_Unit_C|GetPuppet (Variables|Default|GetTargetUnit)))
  (|CallParentFunction))

(event EventPlayAction
  (Audio|PlaySound2D (Variables|Default|GetAttackSound) 1.0 1.0 0.0 0 0)
  (Utilities|IsValid (Variables|Default|GetProjectile)
    (:Is%20Valid
      (bind _returnvalue (Game|SpawnActorfromClass "/Game/AdvancedTurnBasedTileToolkit/Maps/2D/Items/BP_Projectile.BP_Projectile_C" (Transformation|GetActorTransform (Variables|Default|GetSourcePuppet)) "AlwaysSpawn" 0 (Transformation|GetActorLocation (Variables|Default|GetTargetPuppet)) (Variables|Default|GetProjectile) 0))
      (EventDispatchers|BindEventtoOnProjectileHit _returnvalue (delegate Custom|AttackHit)))
    (:Is%20Not%20Valid
      (CallFunction|MeleeStrike))))

(fn ConstructionScript
  (|CallParentFunction))