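; 2D move action for the Advanced Turn Based Tile Toolkit that walks an actor along a path.
; PlayAction clears markers, then a looping timeline lerps MovedActor in X and Y between successive MovePath points, keeping its Z.
; Each finished step plays a sound, and the action ends after the last point.
; ShowTargetMarkerIfAllowed places the target marker at the path's end, visible only to the owning client.
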(event EventPlayAction
  (bind _currentpathindex (Variables|Default|GetCurrentPathIndex))
  (CallFunction|ClearMarkers)
  (Variables|Default|SetGridManagerRef (.GridManager (CallFunction|GetGridManager)))
  (if (> (Utilities|Array|LastIndex (Variables|Default|GetMovePath)) (Variables|Default|GetCurrentPathIndex)) :!label _label
    (bind _movetrack (Timeline|TL_Step PlayFromStart)
      (:Update
        (Transformation|SetActorLocation (Variables|Default|GetMovedActor) (Math|Vector|MakeVector (.x (Math|Vector|Lerp(Vector) (Utilities|Array|Get(acopy) (Variables|Default|GetMovePath) _currentpathindex) (Utilities|Array|Get(acopy) (Variables|Default|GetMovePath) (+ _currentpathindex 1)) _movetrack)) (.y (Math|Vector|Lerp(Vector) (Utilities|Array|Get(acopy) (Variables|Default|GetMovePath) _currentpathindex) (Utilities|Array|Get(acopy) (Variables|Default|GetMovePath) (+ _currentpathindex 1)) _movetrack)) (.z (Transformation|GetActorLocation (Variables|Default|GetMovedActor)))) false false))
      (:Finished
        (Math|Integer|IncrementInt (Variables|Default|GetCurrentPathIndex)
          (:%20%20
            (Audio|PlaySound2D "/Game/AdvancedTurnBasedTileToolkit/Maps/2D/Units/A_Step.A_Step" 1.0 1.0 0.0 0 0)
            (goto _label)))))
    (else
      (CallFunction|EndAction true))))

(event EventDestroyed
  (Actor|DestroyActor))

(fn ConstructionScript
  (|CallParentFunction))

(fn ShowTargetMarkerifAllowed
  (bind _movepath (Variables|Default|GetMovePath))
  (if (Variables|Default|GetbShowTargetMarker)
    (bind _bownedbyclient (CallFunction|IsOwnedbyClient))
    (Rendering|SetVisibility (Variables|Default|GetTargetMarker) _bownedbyclient true)
    (if _bownedbyclient
      (Transformation|SetWorldLocation (Variables|Default|GetTargetMarker) (Utilities|Array|Get(acopy) _movepath (Utilities|Array|LastIndex _movepath)) false false)
      (return true)
      (else
        (return false)))
    (else
      (return false))))