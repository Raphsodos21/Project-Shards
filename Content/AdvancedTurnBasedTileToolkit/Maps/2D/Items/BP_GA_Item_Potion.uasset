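; BP_GA_Item_Potion is a 2D turn-based grid item that heals a player-controlled unit when it interacts with the potion.
; The interaction fires once, ignores AI-controlled units, and immediately adds HealAmount to the unit's health, capped at its maximum.
; It then spawns a BP_Action_QuaffPotion_2D action with the puppet and actual amount healed.
; The potion's destruction is deferred until it is off the action queue.
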(event EventInteract
  (params (TriggeringActor :type Actor%20Object%20Reference) (InteractionType :type EInteract%20Enum :default "NewEnumerator0") (CurrentPathIndex :type Integer))
  (bind _asbp_unit (Utilities|Casting|CastToBP_Unit TriggeringActor))
  (if (not (Variables|/Game/AdvancedTurnBasedTileToolkit/Core/Units/BP_Unit.BP_Unit_C|GetbAIControlled _asbp_unit))
    (Utilities|FlowControl|DoOnce false
      (:Completed
        (Variables|Default|SetHealthPreHeal (Variables|/Game/AdvancedTurnBasedTileToolkit/Core/Units/BP_Unit.BP_Unit_C|GetCurrentHealth _asbp_unit))
        (bind _output_get (Variables|/Game/AdvancedTurnBasedTileToolkit/Core/Units/BP_Unit.BP_Unit_C|SetCurrentHealth _asbp_unit (Math|Float|Min(Float) (Variables|/Game/AdvancedTurnBasedTileToolkit/Core/Units/BP_Unit.BP_Unit_C|GetMaxHealth _asbp_unit) (+ (Variables|/Game/AdvancedTurnBasedTileToolkit/Core/Units/BP_Unit.BP_Unit_C|GetCurrentHealth _asbp_unit) (Variables|Default|GetHealAmount)))))
        (Game|SpawnActorfromClass "/Game/AdvancedTurnBasedTileToolkit/Maps/2D/Actions/BP_Action_QuaffPotion_2D.BP_Action_QuaffPotion_2D_C" (Math|Transform|MakeTransform "0, 0, 0" "0, 0, 0" "1,1,1") "Undefined" 0 (Variables|/Game/AdvancedTurnBasedTileToolkit/Core/Units/BP_Unit.BP_Unit_C|GetPuppet _asbp_unit) (- _output_get (Variables|Default|GetHealthPreHeal)) self -1.0 "NewEnumerator0" 0)
        (CallFunction|DestroyActorwhenOffQueue self)))))

(fn ConstructionScript
  (|CallParentFunction))