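; 2D unit for the turn-based tile toolkit, extending a parent unit with sprite visuals, 2D movement and armor.
; Construction reads the MonsterType data table row to set the sprite, stats, default ability, projectile and sounds.
; Simulated tile entries extend the queued move action's path or spawn a BP_Action_Move_2D to move the puppet.
; Health changes subtract Armor from damage, never turning it into healing, before calling the parent.
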(fn ConstructionScript
  (bind _monstertype (Variables|Default|GetMonsterType))
  (|CallParentFunction)
  (bind _returnvalue (Utilities|GetDataTableRow (.datatable _monstertype) (.rowname _monstertype))
    (:then
      (Variables|Default|SetUnitData _returnvalue)
      (CallFunction|AssignVariablesfromUnitData))))

(fn AssignVariablesfromUnitData
  (bind _unitdata (Variables|Default|GetUnitData))
  (Rendering|Components|Sprite|SetSprite (Variables|Default|GetDisplaySprite) (.sprite _unitdata))
  (Variables|Default|SetMaxAP (.ap _unitdata))
  (Variables|Default|SetCurrentAP (.ap _unitdata))
  (Variables|Default|SetMove (.move _unitdata))
  (Variables|Default|SetRange (.range _unitdata))
  (Variables|Default|SetMaxHealth (.health _unitdata))
  (Variables|Default|SetCurrentHealth (.health _unitdata))
  (Variables|Default|SetDamage (.damage _unitdata))
  (Variables|Default|SetInitiative (.initiative _unitdata))
  (Variables|Default|SetDefaultAbility (.defaultability _unitdata))
  (Variables|Default|SetPathfindingType (.pathfindingtype _unitdata))
  (Variables|Default|SetArmor (.armor _unitdata))
  (Variables|Default|SetProjectile (.projectile _unitdata))
  (Variables|Default|SetAttackSound (.attacksound _unitdata))
  (Variables|Default|SetHitSound (.hitsound _unitdata)))

(fn SimulateEnterTile
  (params (EnteringGridIndex :type Integer) (ExitingGridIndex :type Integer) (PathIndexes :type Array%20of%20Integers))
  (bind _gridmanagerref (Variables|Default|GetGridManagerRef))
  (bind _gridlocations (Variables|/Game/AdvancedTurnBasedTileToolkit/Core/Grid/BP_GridManager.BP_GridManager_C|GetGridLocations _gridmanagerref))
  (CallFunction|QueueorExtendMoveAction (.Value (Utilities|Map|Find _gridlocations ExitingGridIndex)) (.Value (Utilities|Map|Find _gridlocations EnteringGridIndex)))
  (|CallParentFunction EnteringGridIndex ExitingGridIndex PathIndexes)
  (return))

(fn QueueorExtendMoveAction
  (params (MoveSource :type Vector) (MoveTarget :type Vector))
  (bind _actionmanager (CallFunction|GetActionManager))
  (bind _asbp_action_move (Utilities|Casting|CastToBP_Action_Move (Utilities|Array|Get(acopy) (Variables|/Game/AdvancedTurnBasedTileToolkit/Core/BP_ActionManager.BP_ActionManager_C|GetActionQueue _actionmanager) (Variables|/Game/AdvancedTurnBasedTileToolkit/Core/BP_ActionManager.BP_ActionManager_C|GetFillCounter _actionmanager)))
    (:then
      (Utilities|Array|Add (Variables|/Game/AdvancedTurnBasedTileToolkit/Core/Actions/BP_Action_Move.BP_Action_Move_C|GetMovePath _asbp_action_move) MoveTarget))
    (:CastFailed
      (Game|SpawnActorfromClass "/Game/AdvancedTurnBasedTileToolkit/Maps/2D/Actions/BP_Action_Move_2D.BP_Action_Move_2D_C" (Math|Transform|MakeTransform "0, 0, 0" "0, 0, 0" "1,1,1") "AlwaysSpawn" 0 (Utilities|Array|MakeArray MoveSource MoveTarget) (Variables|Default|GetPuppet) true -1.0 "NewEnumerator0" 0)))
  (return))

(fn ModifyHealth
  (params (Change :type Float%20%28single-precision%29) (bAutoAnimate :type Boolean) (EndDelay :type Float%20%28single-precision%29))
  (|CallParentFunction (Math|Float|SelectFloat (Math|Float|Min(Float) (+ Change (Variables|Default|GetArmor)) 0.0) Change (< Change 0.0)) bAutoAnimate EndDelay))