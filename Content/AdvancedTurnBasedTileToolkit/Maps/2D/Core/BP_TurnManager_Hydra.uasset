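; Turn manager variant for the 2D Hydra map of the Advanced Turn Based Tile Toolkit, customizing the game-over message.
; DisplayGameOver shows a victory message on the toolkit HUD when the remaining unit is exactly a BP_Unit_2D_Hydra, and a game-over message otherwise.
; The construction script only calls its parent.
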(event EventDisplayGameOver
  (params (RemainingUnit :type BP%20Unit%20Object%20Reference))
  (bind _asbp_hud_atbtt (Utilities|Casting|CastToBP_HUD_ATBTT (HUD|GetHUD (Game|GetPlayerController 0))))
  (if (== (Utilities|GetClass RemainingUnit) "/Game/AdvancedTurnBasedTileToolkit/Maps/2D/Units/BP_Unit_2D_Hydra.BP_Unit_2D_Hydra_C")
    (Default|DisplayCenterText (Variables|/Game/AdvancedTurnBasedTileToolkit/Core/UI/BP_HUD_ATBTT.BP_HUD_ATBTT_C|GetWbpAtbttRef _asbp_hud_atbtt) "VICTORY!" 0.0)
    (else
      (Default|DisplayCenterText (Variables|/Game/AdvancedTurnBasedTileToolkit/Core/UI/BP_HUD_ATBTT.BP_HUD_ATBTT_C|GetWbpAtbttRef _asbp_hud_atbtt) "GAME OVER" 0.0))))

(fn ConstructionScript
  (|CallParentFunction))