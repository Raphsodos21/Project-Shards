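; 2D grid manager that adds fog of war and tile-triggered object interactions to the turn-based grid.
; On activation it covers the grid in instanced-mesh fog and triggers object interactions when units end movement.
; RevealTiles line-traces tiles in range, wakes unaware stealth units and spawns an action to reveal overlapping fog instances.
; A custom pathfinding step admits only revealed tiles and stops expansion at occupied ones.
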(event Custom|EndOnObjects
  (params (Unit :type BP%20Unit%20Object%20Reference) (GridIndex :type Integer))
  (CallFunction|InteractwithObjects GridIndex Unit 0 true "NewEnumerator0" -1))

(event EventActivateGridManager
  (|CallParentFunction)
  (EventDispatchers|BindEventtoOnUnitEndMovementSimulate (delegate Custom|EndOnObjects))
  (CallFunction|SpawnFogOfWar))

(fn ConstructionScript
  (|CallParentFunction))

(fn RevealTiles
  (params (GridIndex :type Integer))
  (bind _gridindexes (CallFunction|FindVisibleTilesandWallsinRange GridIndex (Variables|Default|GetTileRevealRange)))
  (for _array_element _gridindexes
    (if (.ReturnValue (Utilities|Map|Find (Variables|Default|GetGridUnits) _array_element))
      (if (Variables|/Game/AdvancedTurnBasedTileToolkit/Core/Units/BP_UnitStealthComponent.BP_UnitStealthComponent_C|GetbUnaware (Actor|GetComponentbyClass (.Value (Utilities|Map|Find (Variables|Default|GetGridUnits) _array_element)) "/Game/AdvancedTurnBasedTileToolkit/Core/Units/BP_UnitStealthComponent.BP_UnitStealthComponent_C"))
        (Default|Wake (Actor|GetComponentbyClass (.Value (Utilities|Map|Find (Variables|Default|GetGridUnits) _array_element)) "/Game/AdvancedTurnBasedTileToolkit/Core/Units/BP_UnitStealthComponent.BP_UnitStealthComponent_C"))))
    (if (not (Utilities|Set|Contains (Variables|Default|GetRevealedGridIndexes) _array_element))
      (Utilities|Set|Add (Variables|Default|GetRevealedGridIndexes) _array_element)
      (for _array_element_2 (Class|InstancedStaticMeshComponent|GetInstancesOverlappingSphere (Variables|Default|GetFogOfWar) (CallFunction|GetOffsetWorldLocationatIndex _array_element (Variables|Default|GetFogSphereTraceOffset)) 4e+01 true)
        (Utilities|Array|Add (LocalVariables|GetInstanceIndexes) _array_element_2))))
  (if (> (Utilities|Array|Length (LocalVariables|GetInstanceIndexes)) 0)
    (Game|SpawnActorfromClass "/Game/AdvancedTurnBasedTileToolkit/Maps/2D/Actions/BP_Action_RevealTiles_2D.BP_Action_RevealTiles_2D_C" (Math|Transform|MakeTransform "0, 0, 0" "0, 0, 0" "1,1,1") "AlwaysSpawn" 0 (Variables|Default|GetFogOfWar) (LocalVariables|GetInstanceIndexes) -1.0 "NewEnumerator0" 0)
    (return)))

(fn FindVisibleTilesandWallsinRange
  (params (StartIndex :type Integer) (Range :type Integer))
  (bind _traceforwallsheight (Variables|Default|GetTraceForWallsHeight))
  (bind _inrangetiles (CallFunction|GetIndexesinRange StartIndex Range false false))
  (for _array_element _inrangetiles
    (bind (_outhit _returnvalue) (Collision|LineTraceByChannel (CallFunction|GetOffsetWorldLocationatIndex StartIndex _traceforwallsheight) (CallFunction|GetOffsetWorldLocationatIndex _array_element _traceforwallsheight) (Variables|Default|GetRangeTraceChannel) false 0 "None" false)) ; Do not add tiles that are blocked from sight from collision volumes blocking RangeTrace.
    (if _returnvalue
      (if (Math|Vector|Equal(Vector) (.location _outhit) (.Value (Utilities|Map|Find (Variables|Default|GetGridLocations) _array_element)) (* (Variables|Default|GetTileXSize) 1.42))
        (Utilities|Array|Add (LocalVariables|GetFoundIndexes) _array_element :!label _label))
      (else
        (goto _label))))
  (return (LocalVariables|GetFoundIndexes)))

(fn SearchandAddAdjacentTilesCustom1
  (params (SearchStep :type Integer) (PathsMap :type Map%20of%20Integers%20to%20Structs) (ReachableUnits :type Set%20of%20Integers) (Move :type Integer) (OpenListTiles :type Array%20of%20F%20Pathfinding%20Index%20Structures) (DelayedSearchTiles :type Array%20of%20F%20Pathfinding%20Index%20Structures) (ContinuePathTiles :type Array%20of%20F%20Pathfinding%20Index%20Structures))
  (for _array_element OpenListTiles
    (if (== SearchStep (.cost _array_element)) ; If the parent tile cost is higher than the current search range, do not check now, but re-check next iteration
      (bind _output_get (LocalVariables|SetCurrentEdges (.edges (.Value (Utilities|Map|Find (Variables|Default|GetGridEdges) (.index _array_element))))))
      (bind _keys (Utilities|Map|Keys _output_get))
      (for _array_element_2 _keys
        (if (not (Utilities|Map|Contains PathsMap _array_element_2)) ; Has the node already been searched (if so the cost should be > 0)
          (bind ___ (Utilities|MakeLocalVariable (+ (.Value (Utilities|Map|Find (LocalVariables|GetCurrentEdges) _array_element_2)) (.cost _array_element))))
          (if (<= ___ Move)
            (if (Utilities|Set|Contains (Variables|Default|GetRevealedGridIndexes) _array_element_2)
              (Utilities|Map|Add PathsMap _array_element_2 (Utilities|Struct|MakeFPathfinding ___ (.index _array_element)))
              (if (Utilities|Map|Contains (Variables|Default|GetGridUnits) _array_element_2) ; Prevents units from walking through the spaces of other units\n(a variant that allows for movement through friendly units is\nshown in the Search and add adjacent tiles\n(Pass Through Friendlies) function).
                (Utilities|Set|Add ReachableUnits _array_element_2)
                (else
                  (Utilities|Array|Add (LocalVariables|GetLocalOpenListChildTiles) (Utilities|Struct|MakeFPathfindingIndex _array_element_2 ___ (.index _array_element))))))
            (else
              (Utilities|Array|Add ContinuePathTiles (Utilities|Struct|MakeFPathfindingIndex _array_element_2 ___ (.index _array_element)))))))
      (else
        (Utilities|Array|Add DelayedSearchTiles (Utilities|Struct|MakeFPathfindingIndex (.index _array_element) (.cost _array_element) (.parent _array_element))) ; If the movement cost is too high for this search step, save it for later search steps.
      )))
  (return (LocalVariables|GetLocalOpenListChildTiles)))

(fn SpawnFogOfWar
  (for _index (range 0 (- (* (Variables|Default|GetGridSizeX) (Variables|Default|GetGridSizeY)) 1))
    (Utilities|Array|Add (LocalVariables|GetLocalTransforms) (Math|Transform|MakeTransform (Math|Vector|MakeVector (.x (CallFunction|GetDisplayTileLocationfromIndex _index (Variables|Default|GetGridSizeX) (Variables|Default|GetGridSizeY))) (.y (CallFunction|GetDisplayTileLocationfromIndex _index (Variables|Default|GetGridSizeX) (Variables|Default|GetGridSizeY))) (Variables|Default|GetFogOfWarHeight)) "0, 0, 0" "1.050000,1.050000,1.050000")))
  (Components|InstancedStaticMesh|AddInstances (Variables|Default|GetFogOfWar) (LocalVariables|GetLocalTransforms) false)
  (return))