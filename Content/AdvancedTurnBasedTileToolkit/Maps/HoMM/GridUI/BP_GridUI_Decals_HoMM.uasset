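; Grid UI Blueprint for the HoMM (Heroes of Might and Magic-style) map that draws movement paths as dotted decals.
; Overrides spline path display to spawn dot decals at fixed intervals along PathSpline, plus an arrow decal at the end, oriented from the spline's final segment.
; Tracks spawned decals in DotDecals and destroys them when the path clears; the Color input is unused.
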(event EventBeginPlay
  (|CallParentFunction) ; This node is disabled and will not be called.\nDrag off pins to build functionality.
)

(event Collision|EventActorBeginOverlap
  (params (OtherActor :type Actor%20Object%20Reference))
  (|CallParentFunction OtherActor) ; This node is disabled and will not be called.\nDrag off pins to build functionality.
)

(event EventTick
  (params (DeltaSeconds :type Float%20%28single-precision%29))
  (|CallParentFunction DeltaSeconds) ; This node is disabled and will not be called.\nDrag off pins to build functionality.
)

(fn ConstructionScript
  (|CallParentFunction))

(fn DisplaySplineMeshPath
  (params (bDestroyOldSplineMeshes :type Boolean) (Color :type Linear%20Color%20Structure))
  (bind _pathspline (Variables|Default|GetPathSpline))
  (bind _duration (Variables|/Script/Engine.SplineComponent|GetDuration _pathspline))
  (bind _returnvalue (Spline|GetLocationatTime _pathspline _duration "World" false))
  ;[0.305 0.09894 0] Display Spline Mesh Path
  (if bDestroyOldSplineMeshes
    (CallFunction|ClearSplinePath))
  (LocalVariables|SetLocalTileSize (/ 1e+02 3.0))
  (LocalVariables|SetLastSplineIndex (.ReturnValue (Math|Float|Division(WholeandRemainder) (Spline|GetSplineLength (Variables|Default|GetPathSpline)) (+ (LocalVariables|GetLocalTileSize) 0.1))))
  (for _index (range 0 (- (.ReturnValue (Math|Float|Division(WholeandRemainder) (Spline|GetSplineLength (Variables|Default|GetPathSpline)) (+ (LocalVariables|GetLocalTileSize) 0.1))) 1)) ; Add spline meshes from start to end of the spline
    (LocalVariables|SetLocalIndex _index)
    (bind _returnvalue_2 (Rendering|Decal|SpawnDecalatLocation "/Game/AdvancedTurnBasedTileToolkit/Maps/HoMM/GridUI/M_PathDot.M_PathDot" "100.000000,8.000000,8.000000" (Spline|GetLocationatDistanceAlongSpline (Variables|Default|GetPathSpline) (* _index (LocalVariables|GetLocalTileSize)) "World") "-90.000000,0.000000,0.000000" 0.0))
    (Utilities|Array|Add (Variables|Default|GetDotDecals) _returnvalue_2))
  (bind _returnvalue_3 (Rendering|Decal|SpawnDecalatLocation "/Game/AdvancedTurnBasedTileToolkit/Maps/HoMM/GridUI/MI_PathDotArrow.MI_PathDotArrow" "100.000000,50.000000,50.000000" _returnvalue (Math|Rotator|MakeRotator 0.0 -9e+01 (.Yaw (Math|Rotator|BreakRotator (Math|Rotator|FindLookatRotation _returnvalue (Spline|GetLocationatTime _pathspline (- _duration 0.01) "World" false))))) 0.0))
  (Utilities|Array|Add (Variables|Default|GetDotDecals) _returnvalue_3)
  (return))

(fn ClearSplinePath
  (bind _dotdecals (Variables|Default|GetDotDecals))
  (|CallParentFunction)
  (for _array_element _dotdecals
    (Components|DestroyComponent _array_element))
  (Utilities|Array|Clear _dotdecals)
  (return))