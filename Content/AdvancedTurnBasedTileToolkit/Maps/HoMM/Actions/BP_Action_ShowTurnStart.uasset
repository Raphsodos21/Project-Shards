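; BP_Action_ShowTurnStart is an action in the turn-based toolkit's HoMM map that shows the turn-start animation in the HUD.
; When played, it casts the first player's HUD to the HoMM HUD, waits briefly, then passes Turn to the layout widget's PlayTurnStartAnimation.
; It ends after a second fixed delay rather than an animation-finished callback, or immediately if the cast fails.
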(event EventPlayAction
  (bind _asbp_hud_atbtt_homm (Utilities|Casting|CastToBP_HUD_ATBTT_Homm (HUD|GetHUD (Game|GetPlayerController 0)))
    (:then
      (Utilities|FlowControl|Delay 1.0)
      (Default|PlayTurnStartAnimation (Variables|/Game/AdvancedTurnBasedTileToolkit/Maps/HoMM/Core/BP_HUD_ATBTT_Homm.BP_HUD_ATBTT_Homm_C|GetHommLayoutRef _asbp_hud_atbtt_homm) (Variables|Default|GetTurn))
      (Utilities|FlowControl|Delay 1.0)
      (CallFunction|EndAction true))
    (:CastFailed
      (CallFunction|EndAction true))))

(fn ConstructionScript
  (|CallParentFunction))