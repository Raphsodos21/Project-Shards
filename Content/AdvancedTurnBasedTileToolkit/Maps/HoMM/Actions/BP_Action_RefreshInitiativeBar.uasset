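; BP_Action_RefreshInitiativeBar is a turn-based toolkit action that updates the initiative bar in the HoMM-style map's UI.
; On play, it casts the first player controller's HUD to BP_HUD_ATBTT_Homm and passes its Puppets to the layout's initiative bar widget for a refresh.
; It ends the action immediately afterward, also when the HUD cast fails.
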(event EventPlayAction
  (bind _asbp_hud_atbtt_homm (Utilities|Casting|CastToBP_HUD_ATBTT_Homm (HUD|GetHUD (Game|GetPlayerController 0)))
    (:then
      (Default|RefreshInitiativeBar (Variables|/Game/AdvancedTurnBasedTileToolkit/Maps/HoMM/UI/WBP_Layout_HoMM.WBP_Layout_HoMM_C|GetWBP_InitiativeBar (Variables|/Game/AdvancedTurnBasedTileToolkit/Maps/HoMM/Core/BP_HUD_ATBTT_Homm.BP_HUD_ATBTT_Homm_C|GetHommLayoutRef _asbp_hud_atbtt_homm)) (Variables|Default|GetPuppets))
      (CallFunction|EndAction true))
    (:CastFailed
      (CallFunction|EndAction true))))

(fn ConstructionScript
  (|CallParentFunction))