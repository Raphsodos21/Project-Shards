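; Animated unit blueprint for the HoMM (Heroes of Might and Magic style) example, where each unit is a stack of creatures.
; Damage beyond current health removes creatures from the stack, spawns a HoMM damage action and kills the unit at zero.
; Attacks scale random damage by stack size, and adjacent melee defenders counter once until refreshed.
; Construction lowers initiative by faction index so earlier factions win ties.
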(event EventSetStackSizeHomm
  (params (StackSize :type Integer))
  (Variables|Default|SetStackSize StackSize))

(fn ConstructionScript
  (Variables|Default|SetInitiative (- (Variables|Default|GetInitiative) (* (Math|Conversions|ToInteger(Byte) (Variables|Default|GetFaction)) 0.5))) ; Ensures earlier factions (like the player) wins ties
  (|CallParentFunction))

(fn ModifyHealth
  (params (Change :type Float%20%28single-precision%29) (bAutoAnimate :type Boolean) (EndDelay :type Float%20%28single-precision%29))
  (bind _maxhealth (Variables|Default|GetMaxHealth))
  (if (or (> Change 0.0) (> (+ (Variables|Default|GetCurrentHealth) Change) 0.0))
    (|CallParentFunction Change bAutoAnimate EndDelay)
    (else
      (bind _output_get (Variables|Default|SetStackSize (Math|Integer|Max(Integer) (- (Variables|Default|GetStackSize) (+ (Math|Float|Ceil (/ (Math|Float|Absolute(Float) (+ (Variables|Default|GetCurrentHealth) Change)) _maxhealth)) (Math|Conversions|ToInteger(Boolean) (== (Math|Float|%(Float) (Math|Float|Absolute(Float) (+ (Variables|Default|GetCurrentHealth) Change)) _maxhealth) 0.0)))))))
      (if (== _output_get 0)
        (Variables|Default|SetCurrentHealth 0.0)
        (else
          (Variables|Default|SetCurrentHealth (- (Variables|Default|GetMaxHealth) (Math|Float|%(Float) (Math|Float|Absolute(Float) (+ (Variables|Default|GetCurrentHealth) Change)) (Variables|Default|GetMaxHealth))))))
      (if bAutoAnimate
        (Game|SpawnActorfromClass "/Game/AdvancedTurnBasedTileToolkit/Maps/HoMM/Actions/BP_Action_DealDamageHoMM.BP_Action_DealDamageHoMM_C" (Math|Transform|MakeTransform "0, 0, 0" "0, 0, 0" "1,1,1") "AlwaysSpawn" 0 (Variables|Default|GetPuppet) (Variables|Default|GetCurrentHealth) (Transformation|GetActorLocation (Variables|Default|GetPuppet)) (Variables|Default|GetStackSize) -1.0 "NewEnumerator0" 0))
      (if (== (Variables|Default|GetStackSize) 0)
        (CallFunction|KillUnit)
        (return)
        (else
          (return))))))

(fn QueueAttackAction
  (params (TargetUnit :type BP%20Unit%20Object%20Reference) (bIsRanged :type Boolean))
  (Game|SpawnActorfromClass "/Game/AdvancedTurnBasedTileToolkit/Core/Actions/BP_Action_Attack.BP_Action_Attack_C" (Math|Transform|MakeTransform "0, 0, 0" "0, 0, 0" "1,1,1") "Undefined" 0 (Variables|/Game/AdvancedTurnBasedTileToolkit/Core/Units/BP_Unit.BP_Unit_C|GetPuppet TargetUnit) (Variables|Default|GetPuppet) (select bIsRanged "(TagName=\"Anim.Ranged\")" "(TagName=\"Anim.Attack\")") -1.0 "NewEnumerator0" 0)
  (return))

(fn RefreshUnit
  (|CallParentFunction)
  (Variables|Default|SetbHasCounterAttacked false)
  (return))

(fn DefaultAttackHomm
  (params (TargetUnit :type BP%20Unit%20Object%20Reference) (bIsCounterAttack :type Boolean))
  (bind _damagerange (Variables|Default|GetDamageRange))
  (if (and bIsCounterAttack (or (> (Variables|Default|GetRange) 1) (Variables|Default|GetbHasCounterAttacked)))
    (return false)
    (else
      (CallFunction|QueueAttackAction TargetUnit (> (Default|FindDistanceIinTilesBetweenIndexes (Variables|Default|GetGridManagerRef) (Variables|Default|GetGridIndex) (Variables|/Game/AdvancedTurnBasedTileToolkit/Core/Units/BP_Unit.BP_Unit_C|GetGridIndex TargetUnit) false) 1))
      (CallFunction|ModifyHealth TargetUnit (* (* (Variables|Default|GetStackSize) (Math|Conversions|ToFloat(Integer) (Math|Random|RandomIntegerinRange (Math|Float|Truncate (.x _damagerange)) (Math|Float|Truncate (.y _damagerange))))) -1.0) true (Variables|Default|GetPostHitDelay))
      (if bIsCounterAttack
        (Variables|Default|SetbHasCounterAttacked true))
      (bind _targetunit (LocalVariables|GetTargetUnit)
        (:then
          (if (and (not bIsCounterAttack) (== (Default|FindDistanceIinTilesBetweenIndexes (Variables|Default|GetGridManagerRef) (Variables|Default|GetGridIndex) (Variables|/Game/AdvancedTurnBasedTileToolkit/Core/Units/BP_Unit.BP_Unit_C|GetGridIndex TargetUnit) false) 1))
            (bind _bsuccess (Class|BPIHoMM|DefaultAttackHomm(Message) _targetunit self true))
            (return _bsuccess)
            (else
              _)))
        (:else
          _))
      (return true))))

(fn GetStackSizeHomm
  (return (Variables|Default|GetStackSize)))