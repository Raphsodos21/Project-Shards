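; Grid camera for the experimental hybrid map that animates transitions between the grid view and a third-person character view.
; Two timelines blend camera transform (dual-quaternion interpolation) and FOV, with player input disabled until each finishes.
; Leaving third person snaps the actor to the hybrid puppet character and blends from the supplied view to its reset camera.
; Entering it blends to the pawn's follow camera, then possesses that pawn.
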(event Custom|LerpFromThirdPerson
  (params (ThirdPersonCameraTransform :type Transform) (ThirdPersonFov :type Float%20%28single-precision%29))
  (bind _returnvalue (Game|GetPlayerController 0))
  (bind _returnvalue_2 (Game|GetPlayerController 0))
  (Input|DisableInput _returnvalue _returnvalue)
  (bind _returnvalue_3 (Actor|GetActorOfClass "/Game/AdvancedTurnBasedTileToolkit/Maps/Experimental/Hybrid/BP_Character_Puppet_Hybrid.BP_Character_Puppet_Hybrid_C"))
  (Transformation|SetActorLocation (Transformation|GetActorLocation _returnvalue_3) false false)
  (Transformation|SetRelativeTransform (Variables|Default|GetCamera) (Math|Transform|MakeTransform "0, 0, 0" "0, 0, 0" "1,1,1") false false)
  (bind ___ (Utilities|MakeLocalVariable (Transformation|GetWorldTransform (Variables|Default|GetCamera))))
  (bind _lerptrack (Timeline|TL_CameraLerp PlayFromStart)
    (:Update
      (Transformation|SetWorldTransform (Variables|Default|GetCamera) (Math|Transform|Lerp(Transform) ThirdPersonCameraTransform ___ _lerptrack "DualQuatInterp") false false)
      (Camera|SetFieldOfView (Variables|Default|GetCamera) (Math|Float|Lerp ThirdPersonFov 45.0 _lerptrack)))
    (:Finished
      (Input|EnableInput _returnvalue_2 _returnvalue_2))))

(event Custom|LerpToThirdPersonAndPossess
  (params (ThirdPersonPawn :type BP%20Character%20Puppet%20Hybrid%20Object%20Reference))
  (bind _returnvalue (Game|GetPlayerController 0))
  (bind _returnvalue_2 (Game|GetPlayerController 0))
  (bind _followcamera (Variables|/Game/AdvancedTurnBasedTileToolkit/Maps/Experimental/Hybrid/BP_Character_Puppet_Hybrid.BP_Character_Puppet_Hybrid_C|GetFollowCamera ThirdPersonPawn))
  (Input|DisableInput _returnvalue_2 _returnvalue_2)
  (bind ___ (Utilities|MakeLocalVariable (Variables|/Script/Engine.CameraComponent|GetFieldOfView (Variables|Default|GetCamera))))
  (bind ____2 (Utilities|MakeLocalVariable (Transformation|GetWorldTransform (Variables|Default|GetCamera))))
  (bind _lerptrack (Timeline|TL_CameraLerp2 PlayFromStart)
    (:Update
      (Transformation|SetWorldTransform (Variables|Default|GetCamera) (Math|Transform|Lerp(Transform) ____2 (Transformation|GetWorldTransform _followcamera) _lerptrack "DualQuatInterp") false false)
      (Camera|SetFieldOfView (Variables|Default|GetCamera) (Math|Float|Lerp ___ (Variables|/Script/Engine.CameraComponent|GetFieldOfView _followcamera) _lerptrack)))
    (:Finished
      (Pawn|Possess (Game|GetPlayerController 0) ThirdPersonPawn)
      (Input|EnableInput _returnvalue _returnvalue))))

(fn ConstructionScript
  (|CallParentFunction))