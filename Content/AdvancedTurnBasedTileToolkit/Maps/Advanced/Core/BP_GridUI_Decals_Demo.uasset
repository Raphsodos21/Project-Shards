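; Demo child of the decal-based grid UI in the turn-based tile toolkit, displaying colored movement paths and a matching hover marker.
; DisplayPath calls the parent without clearing the old path, then tints the hover decal's dynamic material to the path color.
; DisplaySplitMovementSpline builds a straight spline with points about 200 units apart and lays raised, color-tinted spline meshes along it, ignoring its DestroyOldSplineMeshes input.
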(event EventBeginPlay
  (|CallParentFunction)
  (bind _returnvalue (Rendering|Material|CreateDynamicMaterialInstance (Variables|Default|GetHoverMarkerDecal) :!class /Script/Engine.DecalComponent))
  (Variables|Default|SetHoverMarkerMaterial _returnvalue))

(event EventDisplayPath
  (params (SplineMeshVectors :type Array%20of%20Vectors) (Color :type Linear%20Color%20Structure) (bClearOldPath :type Boolean))
  (|CallParentFunction SplineMeshVectors Color false)
  (Rendering|Material|SetVectorParameterValue (Variables|Default|GetHoverMarkerMaterial) "Color" Color :!class /Script/Engine.MaterialInstanceDynamic))

(fn ConstructionScript
  (|CallParentFunction))

(fn DisplaySplitMovementSpline
  (params (bDestroyOldSplineMeshes :type Boolean) (StartLocation :type Vector) (EndLocation :type Vector) (Color :type Linear%20Color%20Structure :default "(R=1.000000,G=1.000000,B=1.000000,A=1.000000)") (Mesh :type Static%20Mesh%20Object%20Reference) (Material :type Material%20Interface%20Object%20Reference))
  (bind _splitmovementspline (Variables|Default|GetSplitMovementSpline))
  (bind _splitmovementspline_2 (Variables|Default|GetSplitMovementSpline))
  (bind _returnvalue (Spline|GetNumberOfSplinePoints _splitmovementspline))
  (bind _returnvalue_2 (- StartLocation EndLocation))
  (bind _returnvalue_3 (Spline|GetSplineLength _splitmovementspline))
  (bind _returnvalue_4 (- _returnvalue 1))
  (bind _returnvalue_5 (Math|Vector|VectorLength _returnvalue_2))
  (bind _returnvalue_6 (Math|Conversions|ToFloat(Integer) _returnvalue_4))
  (bind _returnvalue_7 (/ _returnvalue_5 2e+02))
  (bind _returnvalue_8 (/ _returnvalue_3 _returnvalue_6))
  (bind _returnvalue_9 (Math|Float|Round _returnvalue_7))
  (Spline|ClearSplinePoints (Variables|Default|GetSplitMovementSpline) true)
  (for _index (range 0 _returnvalue_9)
    (Spline|AddSplinePoint (Variables|Default|GetSplitMovementSpline) (Math|Vector|Lerp(Vector) StartLocation EndLocation (/ (Math|Conversions|ToFloat(Integer) _index) (Math|Conversions|ToFloat(Integer) _returnvalue_9))) "World" true))
  ;[0.305 0.09894 0] Display Spline Mesh Path
  (for _index_2 (range 0 _returnvalue_4) ; Add spline meshes from start to end of the spline
    (bind _returnvalue_10 (AddComponent|AddSplineMeshComponent false (Math|Transform|MakeTransform "0, 0, 0" "0, 0, 0" (Math|Conversions|ToVector(Float) (Variables|Default|GetTileScaleFactor)))))
    (Components|StaticMesh|SetStaticMesh _returnvalue_10 Mesh)
    (Rendering|Material|SetMaterial _returnvalue_10 0 "/Game/AdvancedTurnBasedTileToolkit/Core/GridUI/M_Emissive_White.M_Emissive_White")
    (Utilities|Array|Add (Variables|Default|GetSplineMeshes) _returnvalue_10)
    (SplineMesh|SetStartandEnd _returnvalue_10 (+ (Spline|GetLocationatDistanceAlongSpline _splitmovementspline_2 (* _index_2 _returnvalue_8) "World") (Math|Vector|MakeVector 0.0 0.0 (Variables|Default|GetSplineHeight))) (* (Spline|GetDirectionatDistanceAlongSpline _splitmovementspline_2 (* _index_2 _returnvalue_8) "World") _returnvalue_8) (+ (Spline|GetLocationatDistanceAlongSpline _splitmovementspline_2 (+ (* _index_2 _returnvalue_8) _returnvalue_8) "World") (Math|Vector|MakeVector 0.0 0.0 (Variables|Default|GetSplineHeight))) (* (Spline|GetDirectionatDistanceAlongSpline _splitmovementspline_2 (+ (* _index_2 _returnvalue_8) _returnvalue_8) "World") _returnvalue_8) true :!class /Script/Engine.SplineMeshComponent)
    (bind _returnvalue_11 (Rendering|Material|CreateDynamicMaterialInstance _returnvalue_10 0 Material "None" :!class /Script/Engine.PrimitiveComponent))
    (Rendering|Material|SetVectorParameterValue _returnvalue_11 "Color" Color :!class /Script/Engine.MaterialInstanceDynamic))
  (return))