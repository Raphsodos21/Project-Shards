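; Turn-based toolkit action that hands execution to an external actor by sending it a PlayExternalAction message.
; If that actor has a BP_ExternalAction_Component, the action binds to its OnExternalActionDone event before sending and ends when that event fires.
; Without the component, it sends the message and ends immediately.
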(event Custom|ProceedAfterInteractDone
  (CallFunction|EndAction true))

(event EventPlayAction
  (bind _externalactor (Variables|Default|GetExternalActor))
  (bind _returnvalue (Actor|GetComponentbyClass _externalactor "/Game/AdvancedTurnBasedTileToolkit/Core/Actions/BP_ExternalAction_Component.BP_ExternalAction_Component_C"))
  (Utilities|IsValid _returnvalue
    (:Is%20Valid
      (EventDispatchers|BindEventtoOnExternalActionDone _returnvalue (delegate Custom|ProceedAfterInteractDone))
      (Class|BPIExternalAction|PlayExternalAction(Message) (Variables|Default|GetExternalActor) :!label _label))
    (:Is%20Not%20Valid
      (Utilities|FlowControl|Sequence
        (:then_0
          (goto _label))
        (:then_1
          (CallFunction|EndAction true))))))

(fn ConstructionScript
  (|CallParentFunction))