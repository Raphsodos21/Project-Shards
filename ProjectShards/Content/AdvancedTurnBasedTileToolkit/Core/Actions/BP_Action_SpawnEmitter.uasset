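; BP_Action_SpawnEmitter is an action in the Advanced Turn Based Tile Toolkit that plays a one-shot particle and sound effect at a given transform.
; When played, it spawns the emitter template with the transform's location, rotation and scale, using configurable auto-destroy and auto-activate flags.
; It plays the sound at the same location, then immediately ends the action without waiting for either effect to finish.
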(event EventPlayAction
  (bind _transform (Variables|Default|GetTransform))
  (Effects|SpawnEmitteratLocation (Variables|Default|GetEmitterTemplate) (.location _transform) (.rotation _transform) (.scale _transform) (Variables|Default|GetbAutoDestroy) "None" (Variables|Default|GetbAutoActivateSystem))
  (Audio|PlaySoundatLocation (Variables|Default|GetSound) (.location (Variables|Default|GetTransform)) "0, 0, 0" 1.0 1.0 0.0 0 0 0)
  (CallFunction|EndAction true))

(fn ConstructionScript
  (|CallParentFunction))