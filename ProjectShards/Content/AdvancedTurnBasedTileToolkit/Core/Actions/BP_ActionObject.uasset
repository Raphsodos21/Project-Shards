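; Base action object for the turn-based tile toolkit, representing one action that an action manager queues and plays.
; Initialize runs the SetupAction hook and queues the object; AnimateAction stores the calling manager and triggers PlayAction.
; EndAction tells the manager to proceed, and skipping routes into it.
; Setup, play and query functions for skipping, destruction and play-with-previous are empty or constant defaults, apparently meant for child overrides.
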(event Custom|PlayAction)

(event Custom|Initialize
  (CallFunction|SetupAction)
  (Class|BPIAction|QueueAction(Message) (Variables|Default|GetActionManager) self))

(event Custom|SetupAction)

(event EventEndAction
  (params (bAutoProceed :type Boolean))
  (Class|BPIAction|ProceedfromOngoingAction(Message) (Variables|Default|GetActionManager) self "NewEnumerator0"))

(event EventAnimateAction
  (params (CallingActionManager :type BP%20Action%20Manager%20Object%20Reference))
  (Variables|Default|SetActionManager CallingActionManager)
  (CallFunction|PlayAction))

(event EventRunonSkipAction
  (CallFunction|EndAction true))

(event EventForcePlayAction
  (CallFunction|PlayAction))

(fn AdvanceandGetNextVectorArraytoManager
  (return 0))

(fn AttemptDestroyAction
  (return true))

(fn CheckifPlayerShouldSkip
  (params (PlayerController :type Player%20Controller%20Object%20Reference))
  (return false))

(fn IsPlaywithPrevious
  (return false))