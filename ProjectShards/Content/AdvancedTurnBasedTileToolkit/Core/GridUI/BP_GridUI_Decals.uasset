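; BP_GridUI_Decals is the decal-based grid UI for the turn-based tile toolkit, displaying tile markers as decals at given locations.
; Spawning and clearing resolve each marker type to its default decal material, then pass it to decal helper functions.
; Clearing works by material, and clearing all markers loops over a hardcoded list of three marker types, noted as a non-urgent TODO.
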(fn ConstructionScript
  (|CallParentFunction))

(fn SpawnTileMarkers
  (params (MarkerType :type ETileMarkerType%20Enum :default "NewEnumerator0") (Locations :type Array%20of%20Vectors))
  (CallFunction|SpawnDecalsatLocations Locations (CallFunction|GetDefaultMarkerDecal MarkerType))
  (return))

(fn ClearTileMarkers
  (params (MarkerType :type ETileMarkerType%20Enum :default "NewEnumerator0"))
  (CallFunction|ClearSpecifiedDecals (CallFunction|GetDefaultMarkerDecal MarkerType))
  (return))

(fn ClearAllTileMarkers
  (for _array_element (Utilities|Array|MakeArray "NewEnumerator0" "NewEnumerator1" "NewEnumerator2")
    (CallFunction|ClearSpecifiedDecals (CallFunction|GetDefaultMarkerDecal _array_element)))
  (return))