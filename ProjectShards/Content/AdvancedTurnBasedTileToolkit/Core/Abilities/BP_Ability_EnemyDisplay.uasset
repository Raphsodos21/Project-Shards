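; Ability that previews an enemy unit's reach on the grid for the active player.
; On activation it takes range settings from the unit's longest-range ability, or from the unit itself without an ability system, then marks visible tiles in range.
; Releasing a click on the unit toggles between this sight range and pathfinding-based move range, which omits occupied tiles.
; Other released clicks on valid tiles fall through to DefaultClick.
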(event Custom|DisplayMoveRange
  (bind _owningunit (Variables|Default|GetOwningUnit))
  (bind _pathsmap (Default|RunPathfinding (Variables|Default|GetGridManagerRef) (Variables|/Game/AdvancedTurnBasedTileToolkit/Core/Units/BP_Unit.BP_Unit_C|GetGridIndex _owningunit) (Variables|/Game/AdvancedTurnBasedTileToolkit/Core/Units/BP_Unit.BP_Unit_C|GetMove _owningunit) (Variables|/Game/AdvancedTurnBasedTileToolkit/Core/Units/BP_Unit.BP_Unit_C|GetPathfindingType _owningunit)))
  (Utilities|Array|Clear (Variables|Default|GetStoredLocations))
  (bind _keys (Utilities|Map|Keys _pathsmap))
  (for _array_element _keys
    (if (not (Utilities|Map|Contains (Variables|/Game/AdvancedTurnBasedTileToolkit/Core/Grid/BP_GridManager.BP_GridManager_C|GetGridUnits (Variables|Default|GetGridManagerRef)) _array_element))
      (Utilities|Array|Add (Variables|Default|GetStoredLocations) (.Value (Utilities|Map|Find (Variables|/Game/AdvancedTurnBasedTileToolkit/Core/Grid/BP_GridManager.BP_GridManager_C|GetGridLocations (Variables|Default|GetGridManagerRef)) _array_element)))))
  (Default|QueueSpawnTileMarkers (Variables|Default|GetGridUIRef) (Variables|Default|GetStoredLocations) "NewEnumerator3")
  (Variables|Default|SetbDisplayingMove true))

(event Custom|DisplaySightRange
  (bind _range (Variables|Default|GetRange))
  (bind _insighttiles (Default|FindTilesinRange (Variables|Default|GetGridManagerRef) (Variables|/Game/AdvancedTurnBasedTileToolkit/Core/Units/BP_Unit.BP_Unit_C|GetGridIndex (Variables|Default|GetOwningUnit)) _range true (Variables|Default|GetbDiamondShapedVisibility) (* _range (Variables|/Game/AdvancedTurnBasedTileToolkit/Core/Grid/BP_GridManager.BP_GridManager_C|GetTileXSize (Variables|Default|GetGridManagerRef))) (Variables|Default|GetMinRange) true))
  (bind _result (Utilities|Set|ToArray _insighttiles))
  (bind _locations (Default|ConvertGridIndexestoLocations (Variables|Default|GetGridManagerRef) _result "0, 0, 0"))
  (Default|QueueSpawnTileMarkers (Variables|Default|GetGridUIRef) _locations "NewEnumerator4")
  (Variables|Default|SetbDisplayingMove false))

(event EventActivate
  (params (bReassess :type Boolean) (OwningActor :type Actor%20Object%20Reference))
  (bind _asbp_unit (Utilities|Casting|CastToBP_Unit OwningActor))
  (Variables|Default|SetOwningUnit _asbp_unit)
  (Actor|SetOwner (Variables|/Game/AdvancedTurnBasedTileToolkit/Core/BP_TurnManager.BP_TurnManager_C|GetActivePlayer (.TurnManager (CallFunction|GetTurnManager))))
  (CallFunction|MulticastSetupGridUIRef)
  (Utilities|FlowControl|Sequence
    (:then_0
      (Utilities|IsValid (Actor|GetComponentbyClass (Variables|Default|GetOwningUnit) "/Game/AdvancedTurnBasedTileToolkit/Core/Units/BP_AbilitySystem.BP_AbilitySystem_C")
        (:Is%20Valid
          (for _array_element (Variables|/Game/AdvancedTurnBasedTileToolkit/Core/Units/BP_AbilitySystem.BP_AbilitySystem_C|GetAbilityRefs (Actor|GetComponentbyClass (Variables|Default|GetOwningUnit) "/Game/AdvancedTurnBasedTileToolkit/Core/Units/BP_AbilitySystem.BP_AbilitySystem_C"))
            (if (> (Variables|/Game/AdvancedTurnBasedTileToolkit/Core/Abilities/BP_Ability.BP_Ability_C|GetRange _array_element) (Variables|Default|GetRange))
              (Variables|Default|SetRange (Variables|/Game/AdvancedTurnBasedTileToolkit/Core/Abilities/BP_Ability.BP_Ability_C|GetRange _array_element))
              (Variables|Default|SetMinRange (Variables|/Game/AdvancedTurnBasedTileToolkit/Core/Abilities/BP_Ability.BP_Ability_C|GetMinRange _array_element))
              (Variables|Default|SetbDiamondShapedVisibility (Variables|/Game/AdvancedTurnBasedTileToolkit/Core/Abilities/BP_Ability.BP_Ability_C|GetbDiamondShapedVisibility _array_element)))))
        (:Is%20Not%20Valid
          (Variables|Default|SetRange (Variables|/Game/AdvancedTurnBasedTileToolkit/Core/Units/BP_Unit.BP_Unit_C|GetRange (Variables|Default|GetOwningUnit)))
          (Variables|Default|SetMinRange (Variables|/Game/AdvancedTurnBasedTileToolkit/Core/Units/BP_Unit.BP_Unit_C|GetMinimumRange (Variables|Default|GetOwningUnit)))
          (Variables|Default|SetbDiamondShapedVisibility (Variables|/Game/AdvancedTurnBasedTileToolkit/Core/Units/BP_Unit.BP_Unit_C|GetbDiamondShapedVisibility (Variables|Default|GetOwningUnit))))))
    (:then_1
      (CallFunction|DisplaySightRange))))

(event EventServerInteract
  (params (bValidTile :type Boolean) (ClickedIndex :type Integer) (Location :type Vector :default "0, 0, 0") (Key :type Key%20Structure) (bReleased :type Boolean) (ClickType :type EClickType%20Enum :default "NewEnumerator0") (CallingPc :type BP%20Player%20Controller%20ATBTT%20Object%20Reference))
  (if bValidTile
    (if bReleased
      (if (== (Variables|/Game/AdvancedTurnBasedTileToolkit/Core/Units/BP_Unit.BP_Unit_C|GetGridIndex (Variables|Default|GetOwningUnit)) ClickedIndex)
        (if (Variables|Default|GetbDisplayingMove)
          (CallFunction|DisplaySightRange)
          (else
            (CallFunction|DisplayMoveRange)))
        (else
          (CallFunction|DefaultClick ClickedIndex Location))))))

(fn ConstructionScript
  (|CallParentFunction))