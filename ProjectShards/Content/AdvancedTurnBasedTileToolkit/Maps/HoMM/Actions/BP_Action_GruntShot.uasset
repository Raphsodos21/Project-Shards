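; BP_Action_GruntShot is a tile-toolkit action in the HoMM map folder that plays a puppet's ranged shot at a target puppet.
; PlayAction animates the source puppet toward the target and waits for its animation event.
; On that event it unbinds, spawns a small explosion at the gun muzzle, then after a short delay a larger one at the target's center, and ends the action.
; It only handles visuals; sound is still a TODO.
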(event Custom|AttackHit
  (params (AnimatingActor :type Actor%20Object%20Reference) (Animation :type Gameplay%20Tag%20Structure))
  (EventDispatchers|UnbindEventfromOnAnimationEvent (Actor|GetComponentbyClass (Variables|Default|GetSourcePuppet) "/Game/AdvancedTurnBasedTileToolkit/Core/Units/BP_PuppetComponent.BP_PuppetComponent_C") (delegate Custom|AttackHit))
  (bind _muzzletransform (Class|BPIUnitHUD|GetGunMuzzle(Message) (Variables|Default|GetSourcePuppet)))
  (Effects|SpawnEmitteratLocation "/Game/AdvancedTurnBasedTileToolkit/Maps/Advanced/Abilities/PS_Explosion.PS_Explosion" (.location _muzzletransform) (.rotation _muzzletransform) "0.500000,0.500000,0.500000") ; TODO: Add sound
  (Utilities|FlowControl|Delay 0.2)
  (bind _location (Class|BPIUnitHUD|GetPuppetCenter(Message) (Variables|Default|GetTargetPuppet)))
  (Effects|SpawnEmitteratLocation "/Game/AdvancedTurnBasedTileToolkit/Maps/Advanced/Abilities/PS_Explosion.PS_Explosion" _location "0, 0, 0" "2.000000,2.000000,2.000000")
  (CallFunction|EndAction true))

(event EventPlayAction
  (EventDispatchers|BindEventtoOnAnimationEvent (Actor|GetComponentbyClass (Variables|Default|GetSourcePuppet) "/Game/AdvancedTurnBasedTileToolkit/Core/Units/BP_PuppetComponent.BP_PuppetComponent_C") (delegate Custom|AttackHit))
  (Class|BPIPuppet|AnimatePuppet(Message) (Variables|Default|GetSourcePuppet) (Variables|Default|GetAnimTag) (Transformation|GetActorLocation (Variables|Default|GetTargetPuppet))))

(fn ConstructionScript
  (|CallParentFunction))