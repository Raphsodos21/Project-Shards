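; Animation component Blueprint for the Grunt unit in the HoMM example of the Advanced Turn Based Tile Toolkit.
; It overrides QueueAttackAction so ranged attacks spawn a BP_Action_GruntShot action from the unit's puppet to the target's puppet, using the Anim.Ranged tag.
; Melee attacks fall through to the parent implementation.
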(event EventBeginPlay
  (|CallParentFunction) ; This node is disabled and will not be called.\nDrag off pins to build functionality.
)

(event Collision|EventActorBeginOverlap
  (params (OtherActor :type Actor%20Object%20Reference)))

(event EventTick
  (params (DeltaSeconds :type Float%20%28single-precision%29)))

(fn ConstructionScript
  (|CallParentFunction))

(fn QueueAttackAction
  (params (TargetUnit :type BP%20Unit%20Object%20Reference) (bIsRanged :type Boolean))
  (if bIsRanged
    (Game|SpawnActorfromClass "/Game/AdvancedTurnBasedTileToolkit/Maps/HoMM/Actions/BP_Action_GruntShot.BP_Action_GruntShot_C" (Math|Transform|MakeTransform "0, 0, 0" "0, 0, 0" "1,1,1") "Undefined" 0 (Variables|/Game/AdvancedTurnBasedTileToolkit/Core/Units/BP_Unit.BP_Unit_C|GetPuppet TargetUnit) (Variables|Default|GetPuppet) "(TagName=\"Anim.Ranged\")" -1.0 "NewEnumerator0" 0)
    (return)
    (else
      (|CallParentFunction TargetUnit bIsRanged))))