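; Player controller for the Heroes of Might and Magic-style (HoMM) map of the turn-based tile toolkit, adding a custom mouse cursor.
; Client setup extends the parent's, waits until BeginPlay is done, then creates the cursor widget and sets it as the default cursor.
; Icon, corner arrow and angle changes are forwarded to that widget through message calls.
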(event EventClientSetup
  (|CallParentFunction)
  (Utilities|DelayWhile (not (Variables|Default|GetbBeginPlayDone)) ; Only continue if references\nhave been set up
    (:Continue
      (bind _returnvalue (UserInterface|CreateWidget (Variables|Default|GetCustomCursorClass) self))
      (bind _output_get (Variables|Default|SetCustomCursor _returnvalue))
      (Class|PlayerController|SetMouseCursorWidget "Default" _output_get))))

(event EventSetCursorAngle
  (params (Angle :type Float%20%28single-precision%29))
  (Class|BPICursor|SetCursorAngle(Message) (Variables|Default|GetCustomCursor) Angle))

(event EventSetCursorIcon
  (params (Icon :type Texture%202D%20Object%20Reference) (bCornerArrow :type Boolean))
  (Class|BPICursor|SetCursorIcon(Message) (Variables|Default|GetCustomCursor) Icon bCornerArrow))

(fn ConstructionScript
  (|CallParentFunction))