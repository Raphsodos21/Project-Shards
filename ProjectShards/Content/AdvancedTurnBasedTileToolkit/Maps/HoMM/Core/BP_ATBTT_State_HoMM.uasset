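; State Blueprint for the HoMM map variant of the Advanced Turn Based Tile Toolkit, supplying the camera's starting transform.
; GetCameraStartTransform halves the sum of the GridManager's bounds origin and extent, then adds a fixed Y offset to form the location.
; Without a valid GridManager, it falls back to the first player pawn's transform.
; The event graph holds no active logic.
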(event EventBeginPlay)

(event EventTick
  (params (DeltaSeconds :type Float%20%28single-precision%29)))

(fn ConstructionScript
  (|CallParentFunction))

(fn GetCameraStartTransform
  (bind _gridmanager (Variables|Default|GetGridManager)
    (:then
      (return (Math|Conversions|ToTransform(Vector) (+ (/ (+ (.Origin (Collision|GetActorBounds _gridmanager false false)) (.BoxExtent (Collision|GetActorBounds _gridmanager false false))) 2.0) "0,150.000000, 0"))))
    (:else
      (return (Transformation|GetActorTransform (Game|Player|GetPlayerPawn 0))))))