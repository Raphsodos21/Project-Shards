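; Base item actor for the 2D maps of the Advanced Turn Based Tile Toolkit, representing an object placed on the grid.
; On BeginPlay it registers itself with the grid manager at its grid index.
; Interact only prints a warning that no interact event is defined, leaving the behavior to child items.
; The action-related functions are stubs that return false or nothing.
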(event EventBeginPlay
  (Default|AddObjecttoGrid (Variables|Default|GetGridManagerRef) self (Variables|Default|GetGridIndex)))

(event EventInteract
  (params (TriggeringActor :type Actor%20Object%20Reference) (InteractionType :type EInteract%20Enum :default "NewEnumerator0") (CurrentPathIndex :type Integer))
  (Development|PrintString (Utilities|String|Append "WARNING: Object " (Utilities|GetDisplayName TriggeringActor) " attempted to interact with Item " (Utilities|GetDisplayName self) ", which has no defined interact event.") true true "(R=1.000000,G=1.000000,B=0.000000,A=1.000000)" 5.0))

(fn ConstructionScript
  (|CallParentFunction))

(fn AdvanceandGetNextVectorArraytoManager
  (return 0))

(fn AttemptDestroyAction
  (return false))

(fn CheckifPlayerShouldSkip
  (params (PlayerController :type Player%20Controller%20Object%20Reference))
  (return false))

(fn IsPlaywithPrevious
  (return false))