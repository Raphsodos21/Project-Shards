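; Pathfinding object for the 2D turn-based tile toolkit that keeps paths to tiles already revealed from fog of war.
; Both pathfinding entry points cast the grid manager to BP_GridManager_2D, cache it, then defer to the parent search.
; The AddTileIfValid override passes a tile to the parent only if its index is in the manager's RevealedGridIndexes, so unrevealed tiles never join the search.
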(fn AddTileifValid
  (params (EdgeIndex :type Integer%20%28by%20ref%29) (TotalCost :type Integer%20%28by%20ref%29) (ParentIndex :type Integer%20%28by%20ref%29) (Move :type Integer%20%28by%20ref%29) (Paths :type Map%20of%20Integers%20to%20Structs) (OpenListChildTiles :type Array%20of%20F%20Pathfinding%20Index%20Structures))
  (if (Utilities|Set|Contains (Variables|/Game/AdvancedTurnBasedTileToolkit/Maps/2D/Core/BP_GridManager_2D.BP_GridManager_2D_C|GetRevealedGridIndexes (Variables|Default|GetGridManager2DRef)) EdgeIndex)
    (|CallParentFunction EdgeIndex TotalCost ParentIndex Move Paths OpenListChildTiles)
    (return)
    (else
      (return))))

(fn RunPathfinding
  (params (StartIndex :type Integer) (MoveRange :type Integer) (GridManager :type BP%20Grid%20Manager%20Object%20Reference))
  (bind _asbp_grid_manager_2d (Utilities|Casting|CastToBP_GridManager_2D GridManager)
    (:then
      (Variables|Default|SetGridManager2DRef _asbp_grid_manager_2d)
      (bind (_pathsmap _pathobject) (|CallParentFunction StartIndex MoveRange GridManager))
      (return _pathsmap _pathobject))
    (:CastFailed
      (return 0 0))))

(fn RunPathfindingUntilIndexFound
  (params (StartIndex :type Integer) (MoveRange :type Integer) (GridManager :type BP%20Grid%20Manager%20Object%20Reference) (TargetGridIndexes :type Array%20of%20Integers))
  (bind _asbp_grid_manager_2d (Utilities|Casting|CastToBP_GridManager_2D GridManager)
    (:then
      (Variables|Default|SetGridManager2DRef _asbp_grid_manager_2d)
      (bind (_bfoundatleastone _foundgridindexes _pathsmap _pathobject) (|CallParentFunction StartIndex MoveRange GridManager TargetGridIndexes))
      (return _bfoundatleastone _foundgridindexes _pathsmap _pathobject))
    (:CastFailed
      (return false 0 0 0))))