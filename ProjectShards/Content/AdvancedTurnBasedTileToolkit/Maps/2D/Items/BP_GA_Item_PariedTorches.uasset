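; Paired-torch interactable item for the 2D maps of the turn-based tile toolkit, which lights torches and triggers bridges.
; The first Interact calls AttemptRaise on every BP_GA_Bridge in the level, then spawns a BP_Action_LightTorches_2D action with itself as the torch actor.
; A DoOnce gate blocks repeat interactions.
; The construction script positions the PairedAnchor from the PairedTorchOffset variable at a fixed height.
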(event EventInteract
  (params (TriggeringActor :type Actor%20Object%20Reference) (InteractionType :type EInteract%20Enum :default "NewEnumerator0") (CurrentPathIndex :type Integer))
  (Utilities|FlowControl|DoOnce false
    (:Completed
      (bind _outactors (Actor|GetAllActorsOfClass "/Game/AdvancedTurnBasedTileToolkit/Maps/2D/Tiles/BP_GA_Bridge.BP_GA_Bridge_C"))
      (for _array_element _outactors
        (Default|AttemptRaise _array_element))
      (Game|SpawnActorfromClass "/Game/AdvancedTurnBasedTileToolkit/Maps/2D/Actions/BP_Action_LightTorches_2D.BP_Action_LightTorches_2D_C" (Math|Transform|MakeTransform "0, 0, 0" "0, 0, 0" "1,1,1") "Undefined" 0 self -1.0 "NewEnumerator0" 0))))

(fn ConstructionScript
  (bind _pairedtorchoffset (Variables|Default|GetPairedTorchOffset))
  (|CallParentFunction)
  (Transformation|SetRelativeLocation (Variables|Default|GetPairedAnchor) (Math|Vector|MakeVector (.x _pairedtorchoffset) (.y _pairedtorchoffset) 22.0) false false))