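; BP_GA_Item_Equip is a 2D ground item that a hero unit picks up and equips by interacting with it.
; Its construction script reads the EquipmentData row handle and sets the Paper sprite to that row's ground sprite.
; On Interact, a BP_Unit_2D_Hero triggers a one-time equip call with the row's data, then the item is destroyed once off the queue.
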(event EventInteract
  (params (TriggeringActor :type Actor%20Object%20Reference) (InteractionType :type EInteract%20Enum :default "NewEnumerator0") (CurrentPathIndex :type Integer))
  (bind _equipmentdata (Variables|Default|GetEquipmentData))
  (bind _asbp_unit_2d_hero_new (Utilities|Casting|CastToBP_Unit_2D_Hero TriggeringActor))
  (Utilities|FlowControl|DoOnce false
    (:Completed
      (bind _returnvalue (Utilities|GetDataTableRow (.datatable _equipmentdata) (.rowname _equipmentdata))
        (:then
          (Default|Equip _asbp_unit_2d_hero_new self _returnvalue)
          (CallFunction|DestroyActorwhenOffQueue self))))))

(fn ConstructionScript
  (bind _equipmentdata (Variables|Default|GetEquipmentData))
  (|CallParentFunction)
  (bind _returnvalue (Utilities|GetDataTableRow (.datatable _equipmentdata) (.rowname _equipmentdata))
    (:then
      (Rendering|Components|Sprite|SetSprite (Variables|Default|GetPaperSprite) (.GroundSprite (Utilities|Struct|BreakFEquipment2D _returnvalue))))))