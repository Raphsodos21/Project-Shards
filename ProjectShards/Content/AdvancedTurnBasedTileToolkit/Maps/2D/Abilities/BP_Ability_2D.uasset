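; Combined move-and-attack ability for 2D units in the turn-based tile toolkit, waking nearby units on activation.
; Player activation caches pathfinding and marks move tiles; hover previews paths, and clicks on revealed tiles move or attack, approaching the target if needed.
; Attacks spawn a BP_Action_Attack_2D and apply damage.
; With no valid target, the unit approaches the closest found unit, or leaves initiative as unaware if none is found.
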(event Custom|ClientClearPath
  (Default|ClearSplinePath (Variables|Default|GetGridUIRef)))

(event Custom|ClientDisplayPath
  (params (PathLocations :type Array%20of%20Vectors))
  (Default|DisplayPath (Variables|Default|GetGridUIRef) PathLocations "(R=1.000000,G=1.000000,B=1.000000,A=1.000000)" false))

(event EventServerHover
  (params (bValidTile :type Boolean) (HoveredTile :type Integer) (Location :type Vector :default "0, 0, 0"))
  (CallFunction|CallClientHoverfromServer bValidTile HoveredTile)
  (CallFunction|ClientClearPath)
  (if bValidTile
    (if (not (Default|CheckifImpassable (Variables|Default|GetGridManagerRef) (Variables|Default|GetHoveredTile)))
      (if (Utilities|Map|Contains (Variables|Default|GetStoredPathsMap) (Variables|Default|GetHoveredTile)) ; Only show path if the current tile has a move cost (e.g. is reachable)
        (if (Utilities|Set|Contains (Variables|/Game/AdvancedTurnBasedTileToolkit/Maps/2D/Core/BP_GridManager_2D.BP_GridManager_2D_C|GetRevealedGridIndexes (Variables|Default|GetGridManager2DRef)) (Variables|Default|GetHoveredTile))
          (bind _pathlocations (Default|FindSplinePathtoGridIndex (Variables|Default|GetGridManagerRef) (Variables|Default|GetStoredPathsMap) (Variables|Default|GetHoveredTile) (Variables|/Game/AdvancedTurnBasedTileToolkit/Core/Units/BP_Unit.BP_Unit_C|GetAnchorOffset (Variables|Default|GetOwningUnit)) 0 "Linear"))
          (CallFunction|ClientDisplayPath _pathlocations))))))

(event EventDeactivate
  (|CallParentFunction)
  (CallFunction|ClientClearPath))

(event EventPlayerActivate
  (params (Unit :type BP%20Unit%20Object%20Reference))
  (bind _owningunit (Variables|Default|GetOwningUnit))
  (bind (_pathsmap _pathobject) (Default|RunPathfinding (Variables|Default|GetGridManagerRef) (Variables|/Game/AdvancedTurnBasedTileToolkit/Core/Units/BP_Unit.BP_Unit_C|GetGridIndex _owningunit) (Variables|/Game/AdvancedTurnBasedTileToolkit/Core/Units/BP_Unit.BP_Unit_C|GetCurrentAP _owningunit) (Variables|/Game/AdvancedTurnBasedTileToolkit/Core/Units/BP_Unit.BP_Unit_C|GetPathfindingType _owningunit)))
  (Variables|Default|SetStoredPathsMap _pathsmap)
  (bind _insighttiles (Default|FindTilesinRange (Variables|Default|GetGridManagerRef) (Variables|/Game/AdvancedTurnBasedTileToolkit/Core/Units/BP_Unit.BP_Unit_C|GetGridIndex (Variables|Default|GetOwningUnit)) (Variables|Default|GetRange) true false 9999999.0 1 false))
  (bind _result (Utilities|Set|Union _insighttiles (Variables|/Game/AdvancedTurnBasedTileToolkit/Core/Pathfinding/BP_Path.BP_Path_C|GetReachableUnitIndexes _pathobject)))
  (Variables|Default|SetPossibleTargets _result)
  (bind _locations (CallFunction|FindMoveLocations (Variables|Default|GetStoredPathsMap)))
  (Default|QueueSpawnTileMarkers (Variables|Default|GetGridUIRef) _locations "NewEnumerator0"))

(event EventActivate
  (params (bReassess :type Boolean) (OwningActor :type Actor%20Object%20Reference))
  (|CallParentFunction bReassess OwningActor)
  (CallFunction|WakeNearbyUnits (Variables|/Game/AdvancedTurnBasedTileToolkit/Core/Units/BP_Unit.BP_Unit_C|GetGridIndex (Variables|Default|GetOwningUnit)) (Variables|Default|GetNoiseRange) (Variables|Default|GetSpotRange)))

(event EventFoundNoValidTarget
  (bind _owningunit (Variables|Default|GetOwningUnit))
  (bind _owningunit_2 (Variables|Default|GetOwningUnit))
  (bind (_btargetfound _closestunitindex _btargetbehindfriendlyunit _distancetoclosesttarget _pathsmap) (Default|FindClosestUnitinMoveRange (Variables|Default|GetGridManagerRef) (Variables|/Game/AdvancedTurnBasedTileToolkit/Core/Units/BP_Unit.BP_Unit_C|GetGridIndex _owningunit_2) (Variables|/Game/AdvancedTurnBasedTileToolkit/Core/Units/BP_Unit.BP_Unit_C|GetMaxSearchRange _owningunit_2) (Variables|/Game/AdvancedTurnBasedTileToolkit/Core/Units/BP_Unit.BP_Unit_C|GetPathfindingType _owningunit_2) (Variables|/Game/AdvancedTurnBasedTileToolkit/Core/Units/BP_Unit.BP_Unit_C|GetAlliedFactions _owningunit_2) true true))
  (if _btargetfound
    (bind _pathindexes (Default|FindPathtoIndex (Variables|Default|GetGridManagerRef) _pathsmap _closestunitindex))
    (bind (_bpathfound _closestindex) (Default|FindReachableIndexClosesttoTarget (Variables|Default|GetGridManagerRef) _pathindexes (Variables|/Game/AdvancedTurnBasedTileToolkit/Core/Units/BP_Unit.BP_Unit_C|GetPathfindingType (Variables|Default|GetOwningUnit)) (Variables|Default|GetPossibleMove) _distancetoclosesttarget _pathsmap))
    (if _bpathfound
      (Variables|Default|SetStoredPathsMap _pathsmap)
      (CallFunction|PayAPCost false)
      (Default|MovetoIndex (Variables|Default|GetOwningUnit) (Variables|Default|GetStoredPathsMap) _closestindex)
      (CallFunction|SignalAbilityExecuted)
      (else
        (CallFunction|DispatchAssessedValue 0.0)))
    (else
      (Utilities|Array|RemoveItem (Variables|/Game/AdvancedTurnBasedTileToolkit/Core/BP_TurnManager.BP_TurnManager_C|GetInitiativeOrderActors (.TurnManager (CallFunction|GetTurnManager))) _owningunit)
      (Variables|/Game/AdvancedTurnBasedTileToolkit/Core/Units/BP_UnitStealthComponent.BP_UnitStealthComponent_C|SetbUnaware (Actor|GetComponentbyClass _owningunit "/Game/AdvancedTurnBasedTileToolkit/Core/Units/BP_UnitStealthComponent.BP_UnitStealthComponent_C") true)
      (CallFunction|DispatchAssessedValue 0.0))))

(event EventServerInteract
  (params (bValidTile :type Boolean) (ClickedIndex :type Integer) (Location :type Vector :default "0, 0, 0") (Key :type Key%20Structure :default "None") (bReleased :type Boolean) (ClickType :type EClickType%20Enum :default "NewEnumerator0") (CallingPc :type BP%20Player%20Controller%20ATBTT%20Object%20Reference))
  (bind _gridmanager2dref (Variables|Default|GetGridManager2DRef))
  (if bValidTile
    (if bReleased
      (switch Utilities|FlowControl|Switch|SwitchonEClickType ClickType
        (:NewEnumerator0
          (if (and (or (Utilities|Map|Contains (Variables|Default|GetStoredPathsMap) (Variables|Default|GetClickedIndex)) (and (<= (Default|FindDistanceIinTilesBetweenIndexes (Variables|Default|GetGridManagerRef) (Variables|/Game/AdvancedTurnBasedTileToolkit/Core/Units/BP_Unit.BP_Unit_C|GetGridIndex (Variables|Default|GetOwningUnit)) (Variables|Default|GetClickedIndex) false) (Variables|Default|GetRange)) (Utilities|Map|Contains (Variables|/Game/AdvancedTurnBasedTileToolkit/Core/Grid/BP_GridManager.BP_GridManager_C|GetGridUnits _gridmanager2dref) (Variables|Default|GetClickedIndex)))) (Utilities|Set|Contains (Variables|/Game/AdvancedTurnBasedTileToolkit/Maps/2D/Core/BP_GridManager_2D.BP_GridManager_2D_C|GetRevealedGridIndexes _gridmanager2dref) (Variables|Default|GetClickedIndex)))
            (Variables|Default|SetMoveTargetIndex (Variables|Default|GetClickedIndex))
            (if (.ReturnValue (Utilities|Map|Find (Variables|/Game/AdvancedTurnBasedTileToolkit/Core/Grid/BP_GridManager.BP_GridManager_C|GetGridUnits (Variables|Default|GetGridManagerRef)) (Variables|Default|GetMoveTargetIndex)))
              (if (!= (.Value (Utilities|Map|Find (Variables|/Game/AdvancedTurnBasedTileToolkit/Core/Grid/BP_GridManager.BP_GridManager_C|GetGridUnits (Variables|Default|GetGridManagerRef)) (Variables|Default|GetMoveTargetIndex))) (Variables|Default|GetOwningUnit))
                (if (<= (Default|FindDistanceIinTilesBetweenIndexes (Variables|Default|GetGridManagerRef) (Variables|/Game/AdvancedTurnBasedTileToolkit/Core/Units/BP_Unit.BP_Unit_C|GetGridIndex (Variables|Default|GetOwningUnit)) (Variables|Default|GetMoveTargetIndex) true) (Variables|Default|GetRange))
                  (bind _bvisible (Default|CheckifTileIsVisiblefromOtherTile (Variables|Default|GetGridManagerRef) (Variables|/Game/AdvancedTurnBasedTileToolkit/Core/Units/BP_Unit.BP_Unit_C|GetGridIndex (Variables|Default|GetOwningUnit)) (Variables|Default|GetMoveTargetIndex) 99999.0 (Variables|Default|GetMinRange) true false))
                  (if _bvisible
                    (CallFunction|PayAPCost false :!label _label)
                    (CallFunction|ExecuteAbility (Variables|Default|GetMoveTargetIndex))
                    (CallFunction|Deactivate)
                    (CallFunction|SignalAbilityExecuted)
                    (elif (Utilities|Map|Contains (Variables|Default|GetStoredPathsMap) (Variables|Default|GetMoveTargetIndex))
                      (bind _pathindexes (Default|FindPathtoIndex (Variables|Default|GetGridManagerRef) (Variables|Default|GetStoredPathsMap) (Variables|Default|GetMoveTargetIndex) :!label _label_2))
                      (if (< (Utilities|Array|Length _pathindexes) 2)
                        (goto _label)
                        (else
                          (Default|MovetoIndex (Variables|Default|GetOwningUnit) (Variables|Default|GetStoredPathsMap) (Utilities|Array|Get(acopy) _pathindexes (- (Utilities|Array|Length _pathindexes) 2)))
                          (goto _label)))))
                  (else
                    (goto _label_2)))
                (else
                  (CallFunction|PayAPCost false)
                  (CallFunction|Deactivate :!label _label_3)
                  (CallFunction|SignalAbilityExecuted)))
              (elif (Utilities|Map|Contains (Variables|Default|GetStoredPathsMap) (Variables|Default|GetMoveTargetIndex))
                (Default|MovetoIndex (Variables|Default|GetOwningUnit) (Variables|Default|GetStoredPathsMap) (Variables|Default|GetMoveTargetIndex))
                (CallFunction|PayMoveAPCost (Variables|Default|GetClickedIndex) (Variables|Default|GetStoredPathsMap) "NewEnumerator3")
                (goto _label_3)))))))))

(event EventBeginPlay
  (|CallParentFunction)
  (bind _asbp_grid_manager_2d (Utilities|Casting|CastToBP_GridManager_2D (.GridManager (CallFunction|GetGridManager))))
  (Variables|Default|SetGridManager2DRef _asbp_grid_manager_2d))

(fn ConstructionScript
  (|CallParentFunction))

(fn FindMoveLocations
  (params (PathsMap :type Map%20of%20Integers%20to%20Structs))
  (bind _keys (Utilities|Map|Keys PathsMap))
  (for _array_element _keys
    (Utilities|Array|Add (LocalVariables|GetLocalLocations) (+ (.Value (Utilities|Map|Find (Variables|/Game/AdvancedTurnBasedTileToolkit/Core/Grid/BP_GridManager.BP_GridManager_C|GetGridLocations (Variables|Default|GetGridManagerRef)) _array_element)) "0, 0,25.000000")))
  (return (LocalVariables|GetLocalLocations)))

(fn ExecuteAbility
  (params (TargetIndexIn :type Integer))
  (|CallParentFunction TargetIndexIn)
  (bind _asbp_unit_2d (Utilities|Casting|CastToBP_Unit_2D (Variables|Default|GetOwningUnit))
    (:then
      (Game|SpawnActorfromClass "/Game/AdvancedTurnBasedTileToolkit/Maps/2D/Actions/BP_Action_Attack_2D.BP_Action_Attack_2D_C" (Math|Transform|MakeTransform "0, 0, 0" "0, 0, 0" "1,1,1") "Undefined" 0 (.Value (Utilities|Map|Find (Variables|/Game/AdvancedTurnBasedTileToolkit/Core/Grid/BP_GridManager.BP_GridManager_C|GetGridUnits (Variables|Default|GetGridManagerRef)) TargetIndexIn)) _asbp_unit_2d -1.0 "NewEnumerator0" 0)
      (Default|ModifyHealth (.Value (Utilities|Map|Find (Variables|/Game/AdvancedTurnBasedTileToolkit/Core/Grid/BP_GridManager.BP_GridManager_C|GetGridUnits (Variables|Default|GetGridManagerRef)) TargetIndexIn)) (* (Variables|Default|GetDamage) -1.0) true 0.2)
      (return true))
    (:CastFailed
      (Development|PrintString "Warning: BP_Ability_2D can only be used by BP_Unit_2D" true true "(R=1.000000,G=1.000000,B=0.000000,A=1.000000)" 6.0)
      (return false))))